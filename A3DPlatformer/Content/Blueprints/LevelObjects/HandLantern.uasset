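; HandLantern is a lantern Blueprint with a point light and a spot light that switch on and off together.
; The LampSwitch event flips the LightLit flag, sets both intensity variables to zero or to fixed lit values, then applies them to the two light components.
; The spot light is brighter than the point light when lit, and the construction script is empty.
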(event `LampSwitch`
  (if (`self.LightLit`)
    (set `self.LightLit` false)
    (set `self.PointLightIntensity` 0.0)
    (set `self.SpotLightInensity` 0.0)
    (else
      (set `self.LightLit` true)
      (set `self.PointLightIntensity` 100.0)
      (set `self.SpotLightInensity` 500.0)))
  (`LightComponent.SetIntensity` (`self.PointLight`) (`self.PointLightIntensity`))
  (`LightComponent.SetIntensity` (`self.SpotLight`) (`self.SpotLightInensity`)))

(fn `UserConstructionScript`)