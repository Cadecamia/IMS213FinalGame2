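; TheGodSkull is a level object that rises as the game's ending sequence and then closes the game.
; RISE plays a timeline that lifts the root component from its starting height.
; When the rise finishes, it shows an EndScream widget with the score from a passed-in Timer reference plus a fixed bonus, then quits after a short delay.
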(event `GetTimerGS`
  (params (Timer :type "/Game/Blueprints/UIElements/Timer Object Reference"))
  (bind _output_get (set `self.TimerReference` Timer)))

(event `self.ReceiveBeginPlay`
  (bind (_returnvalue_x _returnvalue_y _returnvalue_z) (`KismetMathLibrary.BreakVector` (`SceneComponent.K2_GetComponentLocation` (`self.DefaultSceneRoot`))))
  (set `self.startingZ` _returnvalue_z))

(event `RISE`
  (bind _defaultsceneroot (`self.DefaultSceneRoot`))
  (bind (_returnvalue_x _returnvalue_y _returnvalue_z) (`KismetMathLibrary.BreakVector` (`SceneComponent.K2_GetComponentLocation` _defaultsceneroot)))
  (bind (_direction _zchange) (`Timeline|Timeline` :!via `PlayFromStart`)
    (:`Update`
      (`SceneComponent.K2_SetWorldLocation` _defaultsceneroot (`KismetMathLibrary.MakeVector` _returnvalue_x _returnvalue_y (+ (`self.startingZ`) _zchange)) false false))
    (:`Finished`
      (`KismetSystemLibrary.Delay` 3.0)
      (bind _returnvalue (`|CreateWidget` "/Game/Blueprints/UIElements/EndScream.EndScream_C"))
      (`TextBlock.SetText` (`/Game/Blueprints/UIElements/EndScream.FINALSCORE` _returnvalue) (`KismetTextLibrary.Conv_IntToText` (+ (`/Game/Blueprints/UIElements/Timer.CurrentPoints` (stale `GetTimerGS` _output_get)) 20000)))
      (`UserWidget.AddToViewport` _returnvalue 0)
      (`KismetSystemLibrary.Delay` 3.0)
      (`KismetSystemLibrary.QuitGame` null "Quit"))))

(fn `UserConstructionScript`)