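; DangerObject is a moving hazard that ends the run when the first-person character touches it.
; Dir picks one of four world X/Y directions, Tick sweeps the root along it by Speed per frame, and a two-second delay snaps it back to its start, repeating if Loop is set.
; On overlap it shows an EndScream widget with the referenced timer's points, waits three seconds, then reloads the current level.
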(event `GetTimerDO`
  (params (Timer :type "/Game/Blueprints/UIElements/Timer Object Reference"))
  (bind _output_get (set `self.TimerReference` Timer)))

(event `self.ReceiveActorBeginOverlap`
  (params (OtherActor :type "Actor Object Reference"))
  (cast `/Game/FirstPerson/Blueprints/BP_FirstPersonCharacter` OtherActor)
  (bind _returnvalue (`|CreateWidget` "/Game/Blueprints/UIElements/EndScream.EndScream_C"))
  (`TextBlock.SetText` (`/Game/Blueprints/UIElements/EndScream.FINALSCORE` _returnvalue) (`KismetTextLibrary.Conv_IntToText` (`/Game/Blueprints/UIElements/Timer.CurrentPoints` (stale `GetTimerDO` _output_get))))
  (`UserWidget.AddToViewport` _returnvalue 0)
  (`KismetSystemLibrary.Delay` 3.0)
  (bind _returnvalue_2 (`GameplayStatics.GetCurrentLevelName` true))
  (`GameplayStatics.OpenLevel` (`KismetStringLibrary.Conv_StringToName` _returnvalue_2) false))

(event `self.ReceiveTick`
  (params (DeltaSeconds :type "Float (single-precision)"))
  (bind _defaultsceneroot (`self.DefaultSceneRoot`))
  (bind _speed (`self.speed`))
  (bind (_returnvalue_x _returnvalue_y _returnvalue_z) (`KismetMathLibrary.BreakVector` (`SceneComponent.K2_GetComponentLocation` _defaultsceneroot)))
  (`SceneComponent.K2_SetWorldLocation` _defaultsceneroot (`KismetMathLibrary.MakeVector` (+ _returnvalue_x (* (`self.xChange`) _speed)) (+ _returnvalue_y (* (`self.yChange`) _speed)) _returnvalue_z) true false))

(event `self.ReceiveBeginPlay`
  (bind _defaultsceneroot (`self.DefaultSceneRoot`))
  (bind (_returnvalue_x _returnvalue_y _returnvalue_z) (`KismetMathLibrary.BreakVector` (`SceneComponent.K2_GetComponentLocation` _defaultsceneroot)))
  (bind _output_get (set `self.xStart` _returnvalue_x))
  (bind _output_get_2 (set `self.yStart` _returnvalue_y))
  (switch `int` (`self.dir`)
    (:`Default`
      (set `self.yChange` 0.0 :!label _label)
      (`KismetSystemLibrary.Delay` 2.0)
      (`SceneComponent.K2_SetWorldLocation` _defaultsceneroot (`KismetMathLibrary.MakeVector` _output_get _output_get_2 _returnvalue_z) false false :!label _label_2)
      (if (`self.Loop`)
        (`KismetSystemLibrary.Delay` 2.0 :!label _label_3)
        (goto _label_2)))
    (:`0`
      (goto _label))
    (:`1`
      (set `self.xChange` 1.0)
      (goto _label))
    (:`2`
      (set `self.yChange` 1.0)
      (set `self.xChange` 0.0 :!label _label_4)
      (goto _label_3))
    (:`3`
      (set `self.xChange` -1.0)
      (goto _label))
    (:`4`
      (set `self.yChange` -1.0)
      (goto _label_4))))

(fn `UserConstructionScript`)