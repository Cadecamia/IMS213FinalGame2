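; CircleLillyPad is a level object, a lily pad that moves around its placed position, likely in a circle.
; On BeginPlay it stores the starting X and Y, then plays the Rotation timeline from the start.
; Each update offsets the world location by the timeline's AddX and AddY curves scaled by MovementMultiplyer, keeping the current Z.
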(event `self.ReceiveBeginPlay`
  (bind _defaultsceneroot (`self.DefaultSceneRoot`))
  (bind _movementmultiplyer (`self.MovementMultiplyer`))
  (bind (_returnvalue_x _returnvalue_y _returnvalue_z) (`KismetMathLibrary.BreakVector` (`SceneComponent.K2_GetComponentLocation` _defaultsceneroot)))
  (bind _output_get (set `self.startingX` _returnvalue_x))
  (bind _output_get_2 (set `self.startingY` _returnvalue_y))
  (bind (_direction _addx _addy) (`Timeline|Rotation` :!via `PlayFromStart`)
    (:`Update`
      (`SceneComponent.K2_SetWorldLocation` _defaultsceneroot (`KismetMathLibrary.MakeVector` (+ _output_get (* _addx _movementmultiplyer)) (+ _output_get_2 (* _addy _movementmultiplyer)) _returnvalue_z) false false))))

(fn `UserConstructionScript`)