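; Deathplane is a kill-volume actor that ends the run and restarts the level when the first-person character overlaps it.
; GetTimerDP supplies a timer reference, which provides the current points for the final score.
; On overlap it creates an EndScream widget showing that score, then reopens the current level by name after a short delay.
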(event `GetTimerDP`
  (params (Timer :type "/Game/Blueprints/UIElements/Timer Object Reference"))
  (bind _output_get (set `self.TimerReference` Timer)))

(event `self.ReceiveActorBeginOverlap`
  (params (OtherActor :type "Actor Object Reference"))
  (cast `/Game/FirstPerson/Blueprints/BP_FirstPersonCharacter` OtherActor)
  (bind _returnvalue (`|CreateWidget` "/Game/Blueprints/UIElements/EndScream.EndScream_C"))
  (`TextBlock.SetText` (`/Game/Blueprints/UIElements/EndScream.FINALSCORE` _returnvalue) (`KismetTextLibrary.Conv_IntToText` (`/Game/Blueprints/UIElements/Timer.CurrentPoints` (stale `GetTimerDP` _output_get))))
  (`UserWidget.AddToViewport` _returnvalue 0)
  (`KismetSystemLibrary.Delay` 3.0)
  (bind _returnvalue_2 (`GameplayStatics.GetCurrentLevelName` true))
  (`GameplayStatics.OpenLevel` (`KismetStringLibrary.Conv_StringToName` _returnvalue_2) false))

(fn `UserConstructionScript`)