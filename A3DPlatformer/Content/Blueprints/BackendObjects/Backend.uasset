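; Backend actor that plays a 3D creepy song at its root location when play begins.
; The rest of the graph is disconnected and never runs.
; That dormant logic subtracts a timeline-driven amount from the coin count, showing an end screen and reloading the current level after a delay at zero or below.
; Otherwise it increments time, resets points and prints debug values.
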(event `self.ReceiveBeginPlay`
  (`GameplayStatics.PlaySoundAtLocation` "/Game/Imports/Music/CreepySong3D.CreepySong3D" (`SceneComponent.K2_GetComponentLocation` (`self.DefaultSceneRoot`)) (struct) 1.0 1.0 0.0 null null null null))

(fn `UserConstructionScript`)